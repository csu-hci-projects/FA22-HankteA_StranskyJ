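; Player-controlled physics ball for a multi-level campaign, rolled by angular impulses, with a cooldown jump and instant stop.
; BeginPlay saves the spawn transform, adds the HUD and loads Health and Lives from CampaignGameInstance once per level.
; Respawn destroys the ball and spawns a replacement at that transform with one fewer life.
; Tick runs a Delay-based play timer and polls Lives and Win to pause into lose or win menus.
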(event Custom|Lose%20Game
  (bind _returnvalue (Game|SetGamePaused true))
  (Variables|/Script/Engine.PlayerController|SetbShowMouseCursor (Game|GetPlayerController 0) _returnvalue)
  (bind _returnvalue_2 (UserInterface|CreateWidget "/Game/UI/LoseMenu.LoseMenu_C"))
  (UserInterface|Viewport|AddtoViewport _returnvalue_2 0))

(event Custom|Check%20Lives
  (if (not (> (Variables|Default|GetLives) 0))
    (Utilities|FlowControl|Delay 0.5)
    (CallFunction|LoseGame)))

(event Custom|Respawn
  ;[1 1 1] Respawn character
  (Utilities|FlowControl|Delay 1.0)
  (Actor|DestroyActor)
  (bind _output_get (Variables|Default|SetLives (- (Variables|Default|GetLives) 1)))
  (if (<= _output_get 0)
    (bind _output_get_2 (Variables|Default|SetLives 0))
    (Game|SpawnActorfromClass "BP_Ball_C" (Variables|Default|GetSpawnTransform) "Undefined" 0 _output_get_2 0)
    (else
      (Game|SpawnActorfromClass "BP_Ball_C" (Variables|Default|GetSpawnTransform) "Undefined" 0 _output_get 0))))

(event Custom|Win%20Game
  (bind _returnvalue (Game|SetGamePaused true))
  (Variables|/Script/Engine.PlayerController|SetbShowMouseCursor (Game|GetPlayerController 0) _returnvalue)
  (bind _returnvalue_2 (UserInterface|CreateWidget "/Game/UI/WinMenu.WinMenu_C"))
  (UserInterface|Viewport|AddtoViewport _returnvalue_2 0))

(event Custom|Check%20Win
  (if (Variables|Default|GetWin)
    (Utilities|FlowControl|Delay 0.5)
    (CallFunction|WinGame)))

(event EventBeginPlay
  (Utilities|FlowControl|Sequence
    (:then_0
      (bind _ascampaign_game_instance (Utilities|Casting|CastToCampaignGameInstance (Game|GetGameInstance)))
      (bind _returnvalue (Game|GetCurrentLevelName true))
      (switch string _returnvalue
        (:1
          ;[1 1 1] Numbers of lives based on difficulty
          (if (not (Variables|/Game/CampaignGameInstance.CampaignGameInstance_C|GetLoadOnceLevel1 _ascampaign_game_instance))
            (CallFunction|LoadStatusfromPreviousLevel)
            (Variables|/Game/CampaignGameInstance.CampaignGameInstance_C|SetLoadOnceLevel1 _ascampaign_game_instance true)))
        (:2
          (if (not (Variables|/Game/CampaignGameInstance.CampaignGameInstance_C|GetLoadOnceLevel2 _ascampaign_game_instance))
            (CallFunction|LoadStatusfromPreviousLevel)
            (Variables|/Game/CampaignGameInstance.CampaignGameInstance_C|SetLoadOnceLevel2 _ascampaign_game_instance true)))
        (:3
          (if (not (Variables|/Game/CampaignGameInstance.CampaignGameInstance_C|GetLoadOnceLevel3 _ascampaign_game_instance))
            (CallFunction|LoadStatusfromPreviousLevel)
            (Variables|/Game/CampaignGameInstance.CampaignGameInstance_C|SetLoadOnceLevel3 _ascampaign_game_instance true)))
        (:4
          (if (not (Variables|/Game/CampaignGameInstance.CampaignGameInstance_C|GetLoadOnceLevel4 _ascampaign_game_instance))
            (CallFunction|LoadStatusfromPreviousLevel)
            (Variables|/Game/CampaignGameInstance.CampaignGameInstance_C|SetLoadOnceLevel4 _ascampaign_game_instance true)))
        (:5
          (if (not (Variables|/Game/CampaignGameInstance.CampaignGameInstance_C|GetLoadOnceLevel5 _ascampaign_game_instance))
            (CallFunction|LoadStatusfromPreviousLevel)
            (Variables|/Game/CampaignGameInstance.CampaignGameInstance_C|SetLoadOnceLevel5 _ascampaign_game_instance true)))))
    (:then_1
      ;[1 1 1] Save spawn point
      (Variables|Default|SetSpawnTransform (Transformation|GetActorTransform))
      ;[1 1 1] Add user interface
      (bind _returnvalue_2 (UserInterface|CreateWidget "/Game/UI_Main.UI_Main_C"))
      (UserInterface|Viewport|AddtoViewport _returnvalue_2 0))))

(event EventTick
  (params (DeltaSeconds :type Float%20%28single-precision%29))
  (CallFunction|CheckLives)
  (CallFunction|CheckWin)
  (Utilities|FlowControl|Delay 1.0)
  (if (<= (Variables|Default|GetSec) 60)
    (bind _result (Math|Integer|IncrementInt (Variables|Default|GetSec))
      (:%20%20
        (Variables|Default|SetSec _result)))
    (else
      (Variables|Default|SetSec 0)
      (Math|Integer|IncrementInt (Variables|Default|GetMin)))))

(event Input|ActionEvents|InputActionJump
  (params (Key :type Key%20Structure :default "None"))
  (:Pressed
    (if (Variables|Default|GetCanJump)
      (Physics|AddImpulse (Variables|Default|GetSphere) (Math|Vector|MakeVector 0.0 0.0 (Variables|Default|GetJump%20Height)) "None" true)
      (Variables|Default|SetCanJump false)
      (Utilities|FlowControl|Delay 1.0)
      (Variables|Default|SetCanJump true))))

(event Input|ActionEvents|InputActionStop
  (params (Key :type Key%20Structure :default "None"))
  (bind _sphere (Variables|Default|GetSphere))
  (:Pressed
    (Input|DisableInput 0)
    (Class|PrimitiveComponent|SetAllPhysicsLinearVelocity _sphere (Math|Vector|MakeVector 0.0 0.0 0.0) false)
    (Class|PrimitiveComponent|SetAllPhysicsAngularVelocityinDegrees _sphere (Math|Vector|MakeVector 0.0 0.0 0.0) false)
    (Input|EnableInput 0)))

(event Input|ActionEvents|InputActionStartGame
  (params (Key :type Key%20Structure :default "None"))
  (:Pressed
    (Game|OpenLevel(byObjectReference) "/Game/Maps/1.1")))

(event Input|ActionEvents|InputActionStopGame
  (params (Key :type Key%20Structure :default "None"))
  (:Pressed
    (Game|OpenLevel(byObjectReference) "/Game/Maps/IntroMap.IntroMap")))

(event Input|AxisEvents|InputAxisLeftRight
  (params (AxisValue :type Float%20%28single-precision%29))
  (Class|PrimitiveComponent|AddAngularImpulseinDegrees (Variables|Default|GetSphere) (Math|Vector|MakeVector (* AxisValue (Variables|Default|GetMove%20Speed)) 0.0 0.0) "None" true))

(event Input|AxisEvents|InputAxisForwardBack
  (params (AxisValue :type Float%20%28single-precision%29))
  (Class|PrimitiveComponent|AddAngularImpulseinDegrees (Variables|Default|GetSphere) (Math|Vector|MakeVector 0.0 (* AxisValue (Variables|Default|GetMove%20Speed)) 0.0) "None" true))

(fn ConstructionScript)

(fn FalltoDeath
  (Variables|Default|SetHealth 0.0)
  (CallFunction|Respawn))

(fn LoadStatusfromPreviousLevel
  ;[1 1 1] Load variables stored in CampaignGameInstance into BP_Ball
  (bind _ascampaign_game_instance (Utilities|Casting|CastToCampaignGameInstance (Game|GetGameInstance)))
  (Variables|Default|SetHealth (Variables|/Game/CampaignGameInstance.CampaignGameInstance_C|GetHealth _ascampaign_game_instance))
  (Variables|Default|SetLives (Variables|/Game/CampaignGameInstance.CampaignGameInstance_C|GetLives _ascampaign_game_instance)))

(fn StoreStatus
  (bind _ascampaign_game_instance (Utilities|Casting|CastToCampaignGameInstance (Game|GetGameInstance)))
  (Variables|/Game/CampaignGameInstance.CampaignGameInstance_C|SetHealth _ascampaign_game_instance (Variables|Default|GetHealth))
  (Variables|/Game/CampaignGameInstance.CampaignGameInstance_C|SetLives _ascampaign_game_instance (Variables|Default|GetLives)))
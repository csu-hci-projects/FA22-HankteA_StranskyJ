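; BP_Fire is a fire hazard actor that burns the player's BP_Ball while it overlaps, with a P_Fire emitter attached to its mesh on BeginPlay.
; Overlap plays the Burn timeline, restarting it if Health is full, and end overlap stops it.
; Each timeline update writes LoweredHealth to the ball's Health.
; At zero the ball respawns, and the timeline time resets after a short delay.
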(event EventBeginPlay
  ;[1 1 1] Add fire effect
  (Effects|SpawnEmitterAttached "/Game/StarterContent/Particles/P_Fire.P_Fire" (Variables|Default|GetStaticMesh) "None" "0.000000, 0, 0"))

(event Collision|EventActorBeginOverlap
  (params (OtherActor :type Actor%20Object%20Reference))
  ;[1 1 1] BP_Ball is on fire
  (bind _asbp_ball (Utilities|Casting|CastToBP_Ball OtherActor))
  (if (== (Variables|/Game/SuperGrid/StarterPack/Blueprints/BP_Ball.BP_Ball_C|GetHealth _asbp_ball) 1.0)
    (bind _loweredhealth (Timeline|Burn PlayFromStart)
      (:Update
        (bind _output_get (Variables|/Game/SuperGrid/StarterPack/Blueprints/BP_Ball.BP_Ball_C|SetHealth _asbp_ball _loweredhealth))
        (if (<= _output_get 0.0)
          (Default|Respawn _asbp_ball) ; Kill Player
          (Utilities|FlowControl|Delay 1.0) ; Reset burn timer
          (Timeline|Burn SetNewTime))))
    (else
      (Timeline|Burn Play))))

(event Collision|EventActorEndOverlap
  (params (OtherActor :type Actor%20Object%20Reference))
  (bind _loweredhealth (Timeline|Burn Stop)
    (:Update
      (bind _output_get (Variables|/Game/SuperGrid/StarterPack/Blueprints/BP_Ball.BP_Ball_C|SetHealth (stale Collision|EventActorBeginOverlap _asbp_ball) _loweredhealth))
      (if (<= _output_get 0.0)
        (Default|Respawn (stale Collision|EventActorBeginOverlap _asbp_ball)) ; Kill Player
        (Utilities|FlowControl|Delay 1.0) ; Reset burn timer
        (Timeline|Burn SetNewTime)))))

(fn ConstructionScript)
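; BP_Pitfall is a tutorial level hazard that kills the player's ball when it falls in.
; On actor overlap it casts the other actor to BP_Ball and calls FallToDeath on it.
; The construction script scales the Floor component in X and Y from the Size variable divided by 100, keeping Z at 1.
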(event EventBeginPlay)

(event Collision|EventActorBeginOverlap
  (params (OtherActor :type Actor%20Object%20Reference))
  ;[1 1 1] When the player overlaps the pitfall
  (bind _asbp_ball (Utilities|Casting|CastToBP_Ball OtherActor))
  (Default|FalltoDeath _asbp_ball) ; Set health to 0
)

(event EventTick
  (params (DeltaSeconds :type Float%20%28single-precision%29)))

(fn ConstructionScript
  (Utilities|FlowControl|Sequence
    (:then_0
      (Transformation|SetRelativeScale3D (Variables|Default|GetFloor) (CallFunction|GetNormalSize)))))

(fn GetNormalSize
  (bind _size (Variables|Settings|GetSize))
  (bind _returnvalue (/ _size 1e+02))
  (return (Math|Vector|MakeVector (.x _returnvalue) (.y _returnvalue) 1.0)))
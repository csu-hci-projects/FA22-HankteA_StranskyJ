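; BP_Ball is a player-controlled physics ball that rolls and jumps.
; Movement axes apply angular impulses to the Sphere, Jump applies an upward impulse with a one-second cooldown, and Stop resets linear and angular velocity.
; BeginPlay adds the UI_Health widget to the viewport, and FallToDeath sets Health to zero.
; The Start Game and Stop Game inputs only print debug strings.
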(event EventBeginPlay
  (bind _returnvalue (UserInterface|CreateWidget "/Game/UI_Health.UI_Health_C"))
  (UserInterface|Viewport|AddtoViewport _returnvalue 0))

(event Input|ActionEvents|InputActionJump
  (params (Key :type Key%20Structure :default "None"))
  (:Pressed
    (if (Variables|Default|GetCanJump)
      (Physics|AddImpulse (Variables|Default|GetSphere) (Math|Vector|MakeVector 0.0 0.0 (Variables|Default|GetJump%20Height)) "None" true)
      (Variables|Default|SetCanJump false)
      (Utilities|FlowControl|Delay 1.0)
      (Variables|Default|SetCanJump true))))

(event Input|ActionEvents|InputActionStop
  (params (Key :type Key%20Structure :default "None"))
  (bind _sphere (Variables|Default|GetSphere))
  (:Pressed
    (Input|DisableInput 0)
    (Class|PrimitiveComponent|SetAllPhysicsLinearVelocity _sphere (Math|Vector|MakeVector 0.0 0.0 0.0) false)
    (Class|PrimitiveComponent|SetAllPhysicsAngularVelocityinDegrees _sphere (Math|Vector|MakeVector 0.0 0.0 0.0) false)
    (Input|EnableInput 0)))

(event Input|ActionEvents|InputActionStartGame
  (params (Key :type Key%20Structure :default "None"))
  (:Pressed
    (Development|PrintString "Start Game")))

(event Input|ActionEvents|InputActionStopGame
  (params (Key :type Key%20Structure :default "None"))
  (:Pressed
    (Development|PrintString "Stop Game")))

(event Input|AxisEvents|InputAxisLeftRight
  (params (AxisValue :type Float%20%28single-precision%29))
  (Class|PrimitiveComponent|AddAngularImpulseinDegrees (Variables|Default|GetSphere) (Math|Vector|MakeVector (* AxisValue (Variables|Default|GetMove%20Speed)) 0.0 0.0) "None" true))

(event Input|AxisEvents|InputAxisForwardBack
  (params (AxisValue :type Float%20%28single-precision%29))
  (Class|PrimitiveComponent|AddAngularImpulseinDegrees (Variables|Default|GetSphere) (Math|Vector|MakeVector 0.0 (* AxisValue (Variables|Default|GetMove%20Speed)) 0.0) "None" true))

(fn ConstructionScript)

(fn FalltoDeath
  (Variables|Default|SetHealth 0))